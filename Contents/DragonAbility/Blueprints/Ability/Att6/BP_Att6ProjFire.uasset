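; Fire projectile actor for the dragon's Att6 ability that explodes on contact.
; On BeginPlay it spawns a portal effect, attaches a temporary fire trail, loops a sped-up skeletal animation and sets a limited lifespan.
; A timeline drives the Dissolve material parameter on body and tail.
; Each Tick sphere-traces at the mesh sockets, spawning a Niagara explosion and destroying the actor on a hit.
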(fn ConstructionScript)

(event EventTick
  (params (DeltaSeconds :type Float%20%28single-precision%29))
  (Utilities|IsValid (Variables|Default|GetSkeletalMesh)
    (:Is%20Valid
      (for _array_element (Variables|Default|GetSockets)
        (bind _outhits (Collision|MultiSphereTraceForObjects (Transformation|GetSocketLocation (Variables|Default|GetSkeletalMesh) _array_element) (Transformation|GetSocketLocation (Variables|Default|GetSkeletalMesh) _array_element) 5e+01 (Variables|Default|GetObject%20type) true 0 "None"))
        (bind _array_element_2 (Utilities|Array|ForEachLoopwithBreak _outhits)
          (:LoopBody
            (Niagara|SpawnSystematLocation "/Game/DragonAbility/FX/NS/Fire/NS_FireExplosion.NS_FireExplosion" (.location _array_element_2))
            (Actor|DestroyActor)))))))

(event Custom|WorlDiss
  (Utilities|FlowControl|Delay 0.1)
  (bind _vis (Timeline|StartVisiblity PlayFromStart)
    (:Update
      (Rendering|Material|SetScalarParameterValueonMaterials (Variables|Default|GetSkeletalMesh) "Dissolve" _vis))))

(event EventBeginPlay
  (bind _skeletalmesh (Variables|Default|GetSkeletalMesh))
  (Utilities|FlowControl|Sequence
    (:then_0
      (Utilities|FlowControl|Delay 0.1)
      (bind _returnvalue (Effects|SpawnEmitterAttached "/Game/DragonAbility/FX/PS/Fire/P_TrailFire.P_TrailFire" (Variables|Default|GetSkeletalMesh) "0" "0, 0, 0" "0, 0, 0" "1.000000,1.000000,1.000000" "SnapToTargetIncludingScale"))
      (Variables|/Script/Engine.ParticleSystemComponent|SetInstanceParameters _returnvalue (Utilities|Array|MakeArray (Utilities|Struct|MakeParticleSysParam "VertSurfaceActor" "PSPT_Actor" 0.0 0.0 "0.000000,0.000000,0.000000" "0.000000,0.000000,0.000000" "(B=0,G=0,R=0,A=0)" self)))
      (Utilities|FlowControl|Delay 1e+01)
      (Components|Activation|Deactivate _returnvalue))
    (:then_1
      (Actor|SetLifeSpan 1e+01))
    (:then_2
      (Components|Animation|PlayAnimation _skeletalmesh "/Game/DragonAbility/Anim/Att5Loop2.Att5Loop2" true)
      (Components|Timeline|SetPlayRate _skeletalmesh 2.0))
    (:then_3
      (|PortalEffect))
    (:then_4
      (CallFunction|WorlDiss))))