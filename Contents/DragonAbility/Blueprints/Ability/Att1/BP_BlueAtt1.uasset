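; Blue dragon ability actor that plays a one-shot Att1 animation with portal and water trail effects, then destroys itself.
; On BeginPlay it spawns the portal emitter and drives a visibility timeline into the mesh and tail Dissolve parameter.
; A delayed timeline swaps both to a dissolve material and animates "amount".
; In parallel, Trail attaches a mesh-sourced emitter, later deactivates it, hides eye and Niagara effects, and destroys the actor.
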(event Custom|WorlDiss
  (Utilities|FlowControl|Delay 0.1)
  (bind _vis (Timeline|StartVisiblity PlayFromStart)
    (:Update
      (Rendering|Material|SetScalarParameterValueonMaterials (Variables|Default|GetSkeletalMesh) "Dissolve" _vis))))

(event EventBeginPlay
  (bind _skeletalmesh (Variables|Default|GetSkeletalMesh))
  (Utilities|FlowControl|Sequence
    (:then_0
      (Components|Animation|PlayAnimation (Variables|Default|GetSkeletalMesh) "/Game/DragonAbility/Anim/Att1.Att1" false)
      (Utilities|FlowControl|Sequence
        (:then_0
          (Utilities|FlowControl|Delay 1.35)
          (Utilities|FlowControl|Sequence
            (:then_0
              (Rendering|Material|SetMaterial _skeletalmesh 0 "/Game/DragonAbility/Mat_IN/M_BlueDiss_IN.M_BlueDiss_IN")
              (bind _dis (Timeline|Dissolve Play)
                (:Update
                  (Rendering|Material|SetScalarParameterValueonMaterials (Variables|Default|GetSkeletalMesh) "amount" _dis)
                  (Utilities|FlowControl|Delay 1.2)
                  (Actor|DestroyActor))))
            (:then_1
              (Rendering|Material|SetMaterial _skeletalmesh 1 "/Game/DragonAbility/Mat_IN/M_BlueDiss_IN.M_BlueDiss_IN")
              (Timeline|Dissolve Play))
            (:then_2
              (Rendering|Material|SetMaterial _skeletalmesh 2 "/Game/DragonAbility/Mat_IN/M_BlueDiss_IN.M_BlueDiss_IN")
              (Timeline|Dissolve Play))
            (:then_3
              (Rendering|Material|SetMaterial (Variables|Default|GetTail) 0 "/Game/DragonAbility/Mat_IN/M_BlueDiss_IN.M_BlueDiss_IN")
              (Timeline|Dissolve Play))))
        (:then_1
          (|Trail))))
    (:then_1
      (|PortalEffect))
    (:then_2
      (CallFunction|WorlDiss))))

(fn ConstructionScript)