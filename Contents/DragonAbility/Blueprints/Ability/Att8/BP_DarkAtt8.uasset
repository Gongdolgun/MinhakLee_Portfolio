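; Dark dragon Attack 8 ability actor: a purely visual sequence that plays a sped-up attack animation with Niagara effects, then dissolves and removes itself.
; BeginPlay spawns ground and tornado effects at the root and attaches a trail to the mesh.
; After a shared delay, body and tail switch to a timeline-driven dissolve material as a portal spawns.
; The trail deactivates, extra effect components hide, and the actor is destroyed shortly after.
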(event EventBeginPlay
  (bind _skeletalmesh (Variables|Default|GetSkeletalMesh))
  (bind _skeletalmesh_2 (Variables|Default|GetSkeletalMesh))
  (Components|Animation|PlayAnimation _skeletalmesh "/Game/DragonAbility/Anim/Att6Ground2.Att6Ground2" false)
  (Components|Timeline|SetPlayRate _skeletalmesh 2.0)
  (Utilities|FlowControl|Sequence
    (:then_0
      (Utilities|FlowControl|Delay 3.17)
      (Utilities|FlowControl|Sequence
        (:then_0
          (Rendering|Material|SetMaterial _skeletalmesh_2 0 "/Game/DragonAbility/Mat_IN/M_DarkDiss_IN.M_DarkDiss_IN")
          (bind _dis (Timeline|Dissolve Play)
            (:Update
              (Rendering|Material|SetScalarParameterValueonMaterials (Variables|Default|GetSkeletalMesh) "amount" _dis))))
        (:then_1
          (Rendering|Material|SetMaterial _skeletalmesh_2 1 "/Game/DragonAbility/Mat_IN/M_DarkDiss_IN.M_DarkDiss_IN")
          (Timeline|Dissolve Play))
        (:then_2
          (Rendering|Material|SetMaterial _skeletalmesh_2 2 "/Game/DragonAbility/Mat_IN/M_DarkDiss_IN.M_DarkDiss_IN")
          (Timeline|Dissolve Play))
        (:then_3
          (Rendering|Material|SetMaterial (Variables|Default|GetTail) 0 "/Game/DragonAbility/Mat_IN/M_DarkDiss_IN.M_DarkDiss_IN")
          (Timeline|Dissolve Play))))
    (:then_1
      (|Trail))
    (:then_2
      (|Impact))
    (:then_3
      (|Tornado))
    (:then_4
      (Niagara|SpawnSystematLocation "/Game/DragonAbility/FX/NS/Dark/NS_DarkGround.NS_DarkGround" (Transformation|GetWorldLocation (Variables|Default|GetRoot))))))

(fn ConstructionScript)