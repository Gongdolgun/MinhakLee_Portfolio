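; BP_DragonFxCascade is a dragon actor that dresses its Dragon mesh component with a Cascade body-trail effect.
; On BeginPlay it applies one shared material to the first two material slots and spawns the BodyTrail emitter attached to the mesh.
; It passes itself as the VertSurfaceActor instance parameter, the usual hook for emitting particles from a skeletal mesh's vertices or surface.
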(event EventBeginPlay
  (bind _dragon (Variables|Default|GetDragon))
  (bind _material (Variables|Default|GetMaterial))
  (Utilities|FlowControl|Sequence
    (:then_0
      (Rendering|Material|SetMaterial _dragon 0 _material)
      (bind _returnvalue (Effects|SpawnEmitterAttached (Variables|Default|GetBodyTrail) (Variables|Default|GetDragon) "0" "0, 0, 0" "0, 0, 0" "1.000000,1.000000,1.000000" "SnapToTargetIncludingScale"))
      (Variables|/Script/Engine.ParticleSystemComponent|SetInstanceParameters _returnvalue (Utilities|Array|MakeArray (Utilities|Struct|MakeParticleSysParam "VertSurfaceActor" "PSPT_Actor" 0.0 0.0 "0.000000,0.000000,0.000000" "0.000000,0.000000,0.000000" "(B=0,G=0,R=0,A=0)" self))))
    (:then_1
      (Rendering|Material|SetMaterial _dragon 1 _material))))

(fn ConstructionScript)