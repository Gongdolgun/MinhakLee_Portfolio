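; BP_ky_tree4 is a self-destroying magic effect actor built around a destructible mesh, DMKyTree4.
; On BeginPlay, one timeline animates fresnel exponent and color on a dynamic material while a short delay leads into damage that fractures the mesh.
; A second timeline then drives opacity and refraction, with a delay before the actor destroys itself.
; Both delays hang off timeline Update pins rather than Finished.
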(event EventBeginPlay
  (bind _dm_ky_tree4 (Variables|Default|GetDM_ky_tree4))
  (bind _defaultsceneroot (Variables|Default|GetDefaultSceneRoot))
  (bind _returnvalue (Transformation|GetWorldLocation _defaultsceneroot))
  (bind _returnvalue_2 (Rendering|Material|CreateDynamicMaterialInstance (Variables|Default|GetDM_ky_tree4) 0 0 "None" :!class /Script/Engine.PrimitiveComponent))
  (bind (_direction _fresexp _color) (Timeline|Timeline_1 PlayFromStart)
    (:Update
      (Rendering|Material|SetScalarParameterValue _returnvalue_2 "fresExp" _fresexp :!class /Script/Engine.MaterialInstanceDynamic)
      (Rendering|Material|SetVectorParameterValue _returnvalue_2 "color" (Math|Conversions|ToLinearColor(Vector) _color) :!class /Script/Engine.MaterialInstanceDynamic)
      (Utilities|FlowControl|Delay 0.08)
      (Game|Damage|ApplyDamage _dm_ky_tree4 0 0.0 0 0 0 1.0 _returnvalue _returnvalue 1e+04)
      (bind _returnvalue_3 (Rendering|Material|CreateDynamicMaterialInstance _dm_ky_tree4 0 0 "None" :!class /Script/Engine.PrimitiveComponent))
      (bind (_direction_2 _opacity _ref) (Timeline|Timeline_0 Play)
        (:Update
          (Rendering|Material|SetScalarParameterValue _returnvalue_3 "opacity" _opacity :!class /Script/Engine.MaterialInstanceDynamic)
          (Rendering|Material|SetScalarParameterValue _returnvalue_3 "ref" _ref :!class /Script/Engine.MaterialInstanceDynamic)
          (Utilities|FlowControl|Delay 2.0)
          (Actor|DestroyActor))))))

(event Collision|EventActorBeginOverlap
  (params (OtherActor :type Actor%20Object%20Reference)))

(fn ConstructionScript)