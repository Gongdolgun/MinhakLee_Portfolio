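; BP_ky_wave3 is a magic effect actor that spins and moves three wave components, then removes itself.
; On BeginPlay, one timeline yaws the root while its updates play a second timeline that offsets Wave1, Wave2 and Wave3 along their local X.
; When Wave1's relative X drops below zero, all three snap back near the root origin and the actor is destroyed after a short delay.
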(event EventBeginPlay
  (bind _wave1 (Variables|Default|Getwave1))
  (bind _rotation (Timeline|Timeline_0 Play)
    (:Update
      (Transformation|AddLocalRotation (Variables|Default|GetDefaultSceneRoot) (Math|Rotator|MakeRotator 0.0 0.0 (* _rotation (stale EventTick DeltaSeconds))) false false)
      (bind _location (Timeline|Timeline_1 Play)
        (:Update
          (Transformation|AddLocalOffset _wave1 (Math|Vector|MakeVector (* _location (stale EventTick DeltaSeconds)) 0.0 0.0) false false)
          (if (< (.x (Variables|/Script/Engine.SceneComponent|GetRelativeLocation _wave1)) 0.0)
            (Transformation|SetRelativeLocation _wave1 "0, 0,1.000000" false false)
            (Utilities|FlowControl|Delay 2.0)
            (Actor|DestroyActor)))))))

(event Collision|EventActorBeginOverlap
  (params (OtherActor :type Actor%20Object%20Reference)))

(event EventTick
  (params (DeltaSeconds :type Float%20%28single-precision%29)))

(fn ConstructionScript)