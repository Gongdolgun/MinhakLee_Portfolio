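; BP_CPlayer is the player Blueprint, handling HUD setup and two keyboard shortcuts for spawning enemies.
; BeginPlay adds the Minimap, Chaos and Main widgets to the viewport, keeps references to the latter two and plays the Main widget's FadeOut animation.
; J triggers EnemySpawn on every BP_EnemySpawner in the level.
; C destroys an existing BP_CEnemy_Dummy, if any, then spawns one at a hardcoded transform.
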(event EventBeginPlay
  (bind _returnvalue (Game|GetPlayerController 0))
  (Utilities|FlowControl|Sequence
    (:then_0
      (bind _returnvalue_2 (UserInterface|CreateWidget "/Game/Job/Widgets/WDG_Minimap.WDG_Minimap_C" _returnvalue))
      (UserInterface|Viewport|AddtoViewport _returnvalue_2 0))
    (:then_1
      (bind _returnvalue_3 (UserInterface|CreateWidget "/Game/Job/Widgets/WDG_Chaos.WDG_Chaos_C" _returnvalue))
      (bind _output_get (Variables|Default|SetWDG_Chaos _returnvalue_3))
      (UserInterface|Viewport|AddtoViewport _output_get 0))
    (:then_2
      (bind _returnvalue_4 (UserInterface|CreateWidget "/Game/Job/Widgets/WDG_Main.WDG_Main_C" _returnvalue))
      ;[1 1 1] IK 영상찍을때 해제
      (bind _output_get_2 (Variables|Default|SetWDG_Main _returnvalue_4))
      (UserInterface|Viewport|AddtoViewport _output_get_2 0))
    (:then_3
      (UserInterface|Animation|PlayAnimation (Variables|Default|GetWDG_Main) (Variables|/Game/Job/Widgets/WDG_Main.WDG_Main_C|GetFadeOut (Variables|Default|GetWDG_Main)) 0.0 1 "Forward" 1.0 false))))

(event Input|KeyboardEvents|J
  (params (Key :type Key%20Structure :default "None"))
  (:Pressed
    (bind _outactors (Actor|GetAllActorsOfClass "/Game/BP_EnemySpawner.BP_EnemySpawner_C"))
    (for _array_element _outactors
      (Utilities|IsValid _array_element
        (:Is%20Valid
          (Default|EnemySpawn _array_element))))))

(event Input|KeyboardEvents|C
  (params (Key :type Key%20Structure :default "None"))
  (:Pressed
    (bind _returnvalue (Actor|GetActorOfClass "/Game/Enemies/AI_Dummy/BP_CEnemy_Dummy.BP_CEnemy_Dummy_C"))
    (Utilities|IsValid _returnvalue
      (:Is%20Valid
        (Actor|DestroyActor _returnvalue))
      (:Is%20Not%20Valid
        _))
    (Game|SpawnActorfromClass "/Game/Enemies/AI_Dummy/BP_CEnemy_Dummy.BP_CEnemy_Dummy_C" (Math|Transform|MakeTransform "-83210.000000,64550.000000,94590.000000" "0,180.000000, 0" "1,1,1") "Undefined" 0 0)))

(fn ConstructionScript)