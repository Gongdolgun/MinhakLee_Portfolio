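; Level-exit portal actor that sends the player to SunSetMap once the gate has been opened.
; OpenGate runs once, using a timeline to scale up the portal circle and then enabling query collision on the trigger box.
; The box tracks the overlapping player, and pressing G inside destroys skull enemies and enemy swords, plays the HUD's FadeIn animation, then loads the level after a short delay.
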(event OnComponentBeginOverlap(Box)
  (params (OverlappedComponent :type Primitive%20Component%20Object%20Reference) (OtherActor :type Actor%20Object%20Reference) (OtherComp :type Primitive%20Component%20Object%20Reference) (OtherBodyIndex :type Integer) (bFromSweep :type Boolean) (SweepResult :type Hit%20Result%20Structure%20%28by%20ref%29))
  (bind _asbp_cplayer (Utilities|Casting|CastToBP_CPlayer OtherActor))
  (Variables|Default|SetAs%20BP%20CPlayer _asbp_cplayer)
  (Variables|Default|SetIsPlayerIn true))

(event OnComponentEndOverlap(Box)
  (params (OverlappedComponent :type Primitive%20Component%20Object%20Reference) (OtherActor :type Actor%20Object%20Reference) (OtherComp :type Primitive%20Component%20Object%20Reference) (OtherBodyIndex :type Integer))
  (Utilities|Casting|CastToBP_CPlayer OtherActor)
  (Variables|Default|SetAs%20BP%20CPlayer 0)
  (Variables|Default|SetIsPlayerIn false))

(event Custom|OpenGate
  (if (not (Variables|Default|GetIsOpen))
    (Variables|Default|SetIsOpen true)
    (bind _새_트랙_0 (Timeline|타임라인_0 PlayFromStart)
      (:Update
        (Transformation|SetRelativeScale3D (Variables|Default|GetSM_Portal_Circle) (Math|Vector|Lerp(Vector) "0, 0, 0" "2.000000,2.000000,2.000000" _새_트랙_0)))
      (:Finished
        (Collision|SetCollisionEnabled (Variables|Default|GetBox) "QueryOnly")))))

(event Custom|ChangeLevel
  (bind _as_bp_cplayer (Variables|Default|GetAs%20BP%20CPlayer))
  (bind _wdg_main (Variables|/Game/Player/BP_CPlayer.BP_CPlayer_C|GetWDG_Main _as_bp_cplayer))
  (bind _outactors (Actor|GetAllActorsOfClass "/Game/Enemies/AI/BP_CEnemy_Skull.BP_CEnemy_Skull_C"))
  (for _array_element _outactors
    (Actor|DestroyActor _array_element))
  (bind _outactors_2 (Actor|GetAllActorsOfClass "/Game/Job/Weapons/BP_CWeapon_Enemy_Sword.BP_CWeapon_Enemy_Sword_C"))
  (for _array_element_2 _outactors_2
    (Actor|DestroyActor _array_element_2))
  (UserInterface|Animation|PlayAnimation _wdg_main (Variables|/Game/Job/Widgets/WDG_Main.WDG_Main_C|GetFadeIn _wdg_main) 0.0 1 "Forward" 1.0 false)
  (Utilities|FlowControl|Delay 1.0)
  (Game|OpenLevel(byName) "SunSetMap"))

(event EventBeginPlay
  (Input|EnableInput (Game|GetPlayerController 0)))

(event Input|KeyboardEvents|G
  (params (Key :type Key%20Structure :default "None"))
  (:Pressed
    (if (Variables|Default|GetIsPlayerIn)
      (Variables|Default|GetAs%20BP%20CPlayer
        (:then
          (CallFunction|ChangeLevel))
        (:else)))))

(fn ConstructionScript)