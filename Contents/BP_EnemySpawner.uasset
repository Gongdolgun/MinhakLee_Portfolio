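; BP_EnemySpawner is an actor that spawns Skull and Lich enemies at random points inside its box volume.
; The EnemySpawn event spawns LoopCount Skulls and half as many Liches, each yawed along the direction from the spawner to the player.
; The construction script sizes the box from the BoxExtent variable.
; BeginPlay only enables input; a looping timer node is disconnected, and nothing here calls EnemySpawn.
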(event Custom|EnemySpawn
  (for _index (range 1 (Variables|Default|GetLoopCount))
    (Game|SpawnActorfromClass "/Game/Enemies/AI/BP_CEnemy_Skull.BP_CEnemy_Skull_C" (Math|Transform|MakeTransform (Math|Random|RandomPointinBoundingBox (Transformation|GetActorLocation) (Variables|/Script/Engine.BoxComponent|GetBoxExtent (Variables|Default|GetBox))) (Math|Rotator|MakeRotator 0.0 0.0 (.yaw (Math|Rotator|FindLookatRotation (Transformation|GetActorLocation) (Transformation|GetActorLocation (Game|Player|GetPlayerPawn 0))))) "1,1,1") "Undefined" 0 0))
  (for _index_2 (range 1 (/ (Variables|Default|GetLoopCount) 2))
    (Game|SpawnActorfromClass "/Game/Enemies/AI_Lich/BP_CEnemy_Lich.BP_CEnemy_Lich_C" (Math|Transform|MakeTransform (Math|Random|RandomPointinBoundingBox (Transformation|GetActorLocation) (Variables|/Script/Engine.BoxComponent|GetBoxExtent (Variables|Default|GetBox))) (Math|Rotator|MakeRotator 0.0 0.0 (.yaw (Math|Rotator|FindLookatRotation (Transformation|GetActorLocation) (Transformation|GetActorLocation (Game|Player|GetPlayerPawn 0))))) "1,1,1") "Undefined" 0 0)))

(event EventBeginPlay
  (Input|EnableInput (Game|GetPlayerController 0)))

(fn ConstructionScript
  (Components|Box|SetBoxExtent (Variables|Default|GetBox) (Variables|Default|GetBoxExtent) true))